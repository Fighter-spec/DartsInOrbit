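; BP_BiggerTarget is a target actor that awards PlayerBP score when any overlap hits its box, then destroys itself.
; On overlap it swaps to a glow material and pings, then after a short Delay occasionally plays a recorded sound and adds points, doubled with SpeedUpgrade.
; Tick turns the Score component toward the player camera without roll, but the logic that sets and shows its text is disconnected.
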(event `self.ReceiveTick`
  (params (DeltaSeconds :type "Float (single-precision)"))
  (bind _score (`self.Score`))
  (bind _asplayer_bp (cast `/Game/Characters/Input/PlayerBP` (`GameplayStatics.GetPlayerCharacter` 0)))
  (`SceneComponent.K2_SetWorldRotation` _score (`KismetMathLibrary.MakeRotator` 0.0 (.pitch (`KismetMathLibrary.FindLookAtRotation` (`SceneComponent.K2_GetComponentLocation` _score) (`SceneComponent.K2_GetComponentLocation` (`/Game/Characters/Input/PlayerBP.Camera` _asplayer_bp)))) (.yaw (`KismetMathLibrary.FindLookAtRotation` (`SceneComponent.K2_GetComponentLocation` _score) (`SceneComponent.K2_GetComponentLocation` (`/Game/Characters/Input/PlayerBP.Camera` _asplayer_bp))))) false false))

(event `self.Box.OnComponentBeginOverlap`
  (params (OverlappedComponent :type "PrimitiveComponent Object Reference") (OtherActor :type "Actor Object Reference") (OtherComp :type "PrimitiveComponent Object Reference") (OtherBodyIndex :type Integer) (bFromSweep :type Boolean) (SweepResult :type "HitResult Structure (by ref)"))
  (bind _asplayer_bp (cast `/Game/Characters/Input/PlayerBP` (`GameplayStatics.GetPlayerCharacter` 0)))
  (`PrimitiveComponent.SetMaterial` (`self.StaticMesh`) 0 "/Game/Materials/M_Glow1.M_Glow1")
  (`GameplayStatics.PlaySoundAtLocation` "/Game/Sounds/PingCue.PingCue" (`SceneComponent.K2_GetComponentLocation` (`self.StaticMesh`)) (struct) 1.0 1.0 0.0 null null null null)
  (`KismetSystemLibrary.Delay` 0.2)
  (if (< (`KismetMathLibrary.RandomIntegerInRange` 0 10) 2)
    (`GameplayStatics.PlaySound2D` "/Game/Sounds/AlienSounds/New_Recording_794_Cue.New_Recording_794_Cue" 1.0 1.0 0.0 null null))
  (set `/Game/Characters/Input/PlayerBP.Score` (+ (`/Game/Characters/Input/PlayerBP.Score` _asplayer_bp) 50) _asplayer_bp)
  (`KismetSystemLibrary.PrintString` (`KismetStringLibrary.Conv_VectorToString` (`SceneComponent.K2_GetComponentLocation` (`self.StaticMesh`))))
  (bind _asplayer_bp_2 (cast `/Game/Characters/Input/PlayerBP` (`GameplayStatics.GetPlayerCharacter` 0)))
  (if (`/Game/Characters/Input/PlayerBP.SpeedUpgrade?` _asplayer_bp_2)
    (set `/Game/Characters/Input/PlayerBP.Score` (+ (`/Game/Characters/Input/PlayerBP.Score` _asplayer_bp_2) 50) _asplayer_bp_2))
  (`self.K2_DestroyActor` self))

(fn `UserConstructionScript`)
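; BP_PointsPopup is a text actor, named for showing points, that keeps its text turned toward the player's camera.
; Each Tick it casts the player character to PlayerBP and rotates TextRender using the look-at pitch and yaw to that camera, with roll held at zero.
; The graph does not set the text or remove the actor, and a matching rotation calculation for TextRender1 is left unconnected.
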(event `self.ReceiveTick`
  (params (DeltaSeconds :type "Float (single-precision)"))
  (bind _textrender (`self.TextRender`))
  (bind _asplayer_bp (cast `/Game/Characters/Input/PlayerBP` (`GameplayStatics.GetPlayerCharacter` 0)))
  (`SceneComponent.K2_SetWorldRotation` _textrender (`KismetMathLibrary.MakeRotator` 0.0 (.pitch (`KismetMathLibrary.FindLookAtRotation` (`SceneComponent.K2_GetComponentLocation` _textrender) (`SceneComponent.K2_GetComponentLocation` (`/Game/Characters/Input/PlayerBP.Camera` _asplayer_bp)))) (.yaw (`KismetMathLibrary.FindLookAtRotation` (`SceneComponent.K2_GetComponentLocation` _textrender) (`SceneComponent.K2_GetComponentLocation` (`/Game/Characters/Input/PlayerBP.Camera` _asplayer_bp))))) false false))

(fn `UserConstructionScript`)
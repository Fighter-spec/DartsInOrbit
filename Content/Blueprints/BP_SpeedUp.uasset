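; BP_SpeedUp is a speed-boost pickup that awards score and grants the player a timed speed upgrade.
; Any box overlap destroys the trigger, adds score to player character 0, glows the mesh and plays a ping.
; After a brief delay it hides the pickup, sets SpeedUpgrade and recolors the player's indicators.
; Twenty seconds later it clears the flag and destroys itself, without restoring the indicator materials.
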(event `self.Box.OnComponentBeginOverlap`
  (params (OverlappedComponent :type "PrimitiveComponent Object Reference") (OtherActor :type "Actor Object Reference") (OtherComp :type "PrimitiveComponent Object Reference") (OtherBodyIndex :type Integer) (bFromSweep :type Boolean) (SweepResult :type "HitResult Structure (by ref)"))
  (bind _asplayer_bp (cast `/Game/Characters/Input/PlayerBP` (`GameplayStatics.GetPlayerCharacter` 0)))
  (`ActorComponent.K2_DestroyComponent` (`self.Box`))
  (set `/Game/Characters/Input/PlayerBP.Score` (+ (`/Game/Characters/Input/PlayerBP.Score` _asplayer_bp) 75) _asplayer_bp)
  (`PrimitiveComponent.SetMaterial` (`self.StaticMesh`) 0 "/Game/Materials/M_Glow1.M_Glow1")
  (`GameplayStatics.PlaySoundAtLocation` "/Game/Sounds/PingCue.PingCue" (`SceneComponent.K2_GetComponentLocation` (`self.StaticMesh`)) (struct) 1.0 1.0 0.0 null null null null)
  (`KismetSystemLibrary.Delay` 0.2)
  (bind _asplayer_bp_2 (cast `/Game/Characters/Input/PlayerBP` (`GameplayStatics.GetPlayerCharacter` 0)))
  (set `/Game/Characters/Input/PlayerBP.SpeedUpgrade?` true _asplayer_bp_2)
  (`SceneComponent.SetVisibility` (`self.StaticMesh`) false false)
  (`SceneComponent.SetVisibility` (`self.Cube7`) false false)
  (`SceneComponent.SetVisibility` (`self.Cube4`) false false)
  (`SceneComponent.SetVisibility` (`self.Cube5`) false false)
  (`SceneComponent.SetVisibility` (`self.Cube6`) false false)
  (`SceneComponent.SetVisibility` (`self.Cube3`) false false)
  (`SceneComponent.SetVisibility` (`self.Cube2`) false false)
  (`SceneComponent.SetVisibility` (`self.PointLight`) false false)
  (`SceneComponent.SetVisibility` (`self.PointLight1`) false false)
  (`SceneComponent.SetVisibility` (`self.PointLight2`) false false)
  (`SceneComponent.SetVisibility` (`self.Cube1`) false false)
  (`SceneComponent.SetVisibility` (`self.Cube8`) false false)
  (`SceneComponent.SetVisibility` (`self.Cube9`) false false)
  (`SceneComponent.SetVisibility` (`self.Cube10`) false false)
  (`SceneComponent.SetVisibility` (`self.Cube11`) false false)
  (`SceneComponent.SetVisibility` (`self.Cone5`) false false)
  (`SceneComponent.SetVisibility` (`self.Cube`) false false)
  (`SceneComponent.SetVisibility` (`self.Cone4`) false false)
  (`SceneComponent.SetVisibility` (`self.Cone3`) false false)
  (`SceneComponent.SetVisibility` (`self.Cone`) false false)
  (`SceneComponent.SetVisibility` (`self.Cone1`) false false)
  (`SceneComponent.SetVisibility` (`self.Cone2`) false false)
  (`ActorComponent.K2_DestroyComponent` (`self.PointLight1`))
  (`ActorComponent.K2_DestroyComponent` (`self.PointLight2`))
  (`ActorComponent.K2_DestroyComponent` (`self.PointLight`))
  (`ActorComponent.K2_DestroyComponent` (`self.Sphere`))
  (`PrimitiveComponent.SetMaterial` (`/Game/Characters/Input/PlayerBP.Direction Indicator` _asplayer_bp_2) 0 "/Game/Materials/M_Speedup.M_Speedup")
  (`PrimitiveComponent.SetMaterial` (`/Game/Characters/Input/PlayerBP.Indicator` _asplayer_bp_2) 0 "/Game/Materials/M_Speedup.M_Speedup")
  (`PrimitiveComponent.SetMaterial` (`/Game/Characters/Input/PlayerBP.RingCut` _asplayer_bp_2) 0 "/Game/Materials/M_Speedup.M_Speedup")
  (`KismetSystemLibrary.Delay` 20.0)
  (cast `/Game/Characters/Input/PlayerBP` (`GameplayStatics.GetPlayerCharacter` 0))
  (set `/Game/Characters/Input/PlayerBP.SpeedUpgrade?` false _asplayer_bp_2)
  (`self.K2_DestroyActor` self))

(fn `UserConstructionScript`)
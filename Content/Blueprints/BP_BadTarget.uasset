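; BP_BadTarget is a penalty target that costs the player score when its Box is overlapped.
; The overlap turns the mesh black and four text renders red, plays a failure sound, then after a short delay deducts score, doubles the penalty with SpeedUpgrade, and destroys itself.
; The handler casts player character 0 to PlayerBP rather than checking the overlapping actor, so any overlapping object can trigger it.
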(event `self.Box.OnComponentBeginOverlap`
  (params (OverlappedComponent :type "PrimitiveComponent Object Reference") (OtherActor :type "Actor Object Reference") (OtherComp :type "PrimitiveComponent Object Reference") (OtherBodyIndex :type Integer) (bFromSweep :type Boolean) (SweepResult :type "HitResult Structure (by ref)"))
  (bind _asplayer_bp (cast `/Game/Characters/Input/PlayerBP` (`GameplayStatics.GetPlayerCharacter` 0)))
  (if true
    (`PrimitiveComponent.SetMaterial` (`self.StaticMesh`) 0 "/Engine/MapTemplates/Sky/M_BlackBackground.M_BlackBackground")
    (`PrimitiveComponent.SetMaterial` (`self.TextRender2`) 0 "/AnimationSharing/AnimSharingRed.AnimSharingRed")
    (`PrimitiveComponent.SetMaterial` (`self.TextRender1`) 0 "/AnimationSharing/AnimSharingRed.AnimSharingRed")
    (`PrimitiveComponent.SetMaterial` (`self.TextRender`) 0 "/AnimationSharing/AnimSharingRed.AnimSharingRed")
    (`PrimitiveComponent.SetMaterial` (`self.TextRender3`) 0 "/AnimationSharing/AnimSharingRed.AnimSharingRed")
    (`GameplayStatics.PlaySoundAtLocation` "/Engine/EditorSounds/Notifications/CompileFailed_Cue.CompileFailed_Cue" (`SceneComponent.K2_GetComponentLocation` (`self.StaticMesh`)) (struct) 1.0 1.0 0.0 null null null null)
    (`KismetSystemLibrary.Delay` 0.2)
    (set `/Game/Characters/Input/PlayerBP.Score` (+ (`/Game/Characters/Input/PlayerBP.Score` _asplayer_bp) -50) _asplayer_bp)
    (bind _asplayer_bp_2 (cast `/Game/Characters/Input/PlayerBP` (`GameplayStatics.GetPlayerCharacter` 0)))
    (if (`/Game/Characters/Input/PlayerBP.SpeedUpgrade?` _asplayer_bp_2)
      (set `/Game/Characters/Input/PlayerBP.Score` (+ (`/Game/Characters/Input/PlayerBP.Score` _asplayer_bp_2) -50) _asplayer_bp_2))
    (`self.K2_DestroyActor` self)))

(fn `UserConstructionScript`)